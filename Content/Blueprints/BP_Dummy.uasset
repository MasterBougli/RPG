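; BP_Dummy is a target character that can be stealth-assassinated from behind.
; An overlap radius shows a prompt widget while the third-person character is inside, and Tick rotates the visible widget toward the player camera.
; StealthBackAssassination plays the paired victim knife montage, removes the widget and radius, triggers a delayed ragdoll, and returns a reference location and the dummy's rotation for the caller.
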(event `Ragdoll`
  (`KismetSystemLibrary.Delay` 2.5)
  (`PrimitiveComponent.SetSimulatePhysics` (`self.Mesh`) true))

(event `self.Assassination Radius.OnComponentBeginOverlap`
  (params (OverlappedComponent :type "PrimitiveComponent Object Reference") (OtherActor :type "Actor Object Reference") (OtherComp :type "PrimitiveComponent Object Reference") (OtherBodyIndex :type Integer) (bFromSweep :type Boolean) (SweepResult :type "HitResult Structure (by ref)"))
  (cast `/Game/ThirdPerson/Blueprints/BP_ThirdPersonCharacter` OtherActor)
  (`/Engine/EditorBlueprintResources/StandardMacros.IsValid` (`self.Widget`)
    (:`Is Valid`
      (`SceneComponent.SetVisibility` (`self.Widget`) true false))))

(event `self.Assassination Radius.OnComponentEndOverlap`
  (params (OverlappedComponent :type "PrimitiveComponent Object Reference") (OtherActor :type "Actor Object Reference") (OtherComp :type "PrimitiveComponent Object Reference") (OtherBodyIndex :type Integer))
  (cast `/Game/ThirdPerson/Blueprints/BP_ThirdPersonCharacter` OtherActor)
  (`/Engine/EditorBlueprintResources/StandardMacros.IsValid` (`self.Widget`)
    (:`Is Valid`
      (`SceneComponent.SetVisibility` (`self.Widget`) false false))))

(event `self.ReceiveTick`
  (params (DeltaSeconds :type "Float (single-precision)"))
  (bind _widget (`self.Widget`))
  (`|ExecutionSequence`
    (:`then_0`
      (`/Engine/EditorBlueprintResources/StandardMacros.IsValid` _widget
        (:`Is Valid`
          (if (`SceneComponent.IsVisible` _widget)
            (`self.RotateWidgetAssassin`)))))))

(fn `RotateWidgetAssassin`
  (`SceneComponent.K2_SetWorldRotation` (`self.Widget`) (`KismetMathLibrary.FindLookAtRotation` (`SceneComponent.K2_GetComponentLocation` (`self.Widget`)) (`SceneComponent.K2_GetComponentLocation` (`PlayerCameraManager.TransformComponent` (`GameplayStatics.GetPlayerCameraManager` 0)))) false false))

(fn `Stealth Back Assassination`
  (returns (Ref_Location :type "Vector Structure") (Ref_Rotation :type "Rotator Structure"))
  (`self.PlayAnimMontage` "/Game/Characters/RPG_Character/Animation/Assassination/Paired_Knife_Stealth_KidneyAndNeck_Vic_Montage.Paired_Knife_Stealth_KidneyAndNeck_Vic_Montage")
  (`ActorComponent.K2_DestroyComponent` (`self.Widget`))
  (`ActorComponent.K2_DestroyComponent` (`self.Assassination Radius`))
  (`self.Ragdoll`)
  (return (`SceneComponent.K2_GetComponentLocation` (`self.Ref_Assassin`)) (`self.K2_GetActorRotation`)))

(fn `UserConstructionScript`)