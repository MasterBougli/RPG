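; Attack component for BP_ThirdPersonCharacter that runs a four-step melee combo of two sword attacks, a kick and a final attack.
; IA_Attack starts the chain when allowed, and presses during an attack are buffered in SaveAttack.
; Each step plays its montage after a short DoOnce-guarded delay and advances AttackIndex.
; SwordAttackCombo, called from outside this graph, consumes the buffered press to continue or calls StopCombo to reset.
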(event `self.ReceiveBeginPlay`
  (bind _asbp_third_person_character (cast `/Game/ThirdPerson/Blueprints/BP_ThirdPersonCharacter` (`self.GetOwner`)))
  (set `self.Ref_CharacterMesh` (`Character.Mesh` _asbp_third_person_character)))

(event `Attack1`
  (`/Engine/EditorBlueprintResources/StandardMacros.DoOnce` false :!label _label
    (:`Completed`
      (`KismetSystemLibrary.Delay` 0.1)
      (`|PlayMontage` (`self.Ref_CharacterMesh`) "/Game/Characters/RPG_Character/Animation/SwordAttack/M_Attack1.M_Attack1"
        (:`then`
          (set `self.AttackIndex` 1)
          (goto _label :!via `Reset`))))))

(event `EnhancedInput|/Game/ThirdPerson/Input/Actions/IA_Attack`
  (params (ActionValue :type Boolean) (ElapsedSeconds :type "Float (double-precision)") (TriggeredSeconds :type "Float (double-precision)") (InputAction :type "InputAction Object Reference" :default "/Game/ThirdPerson/Input/Actions/IA_Attack.IA_Attack"))
  (:`Started`
    (if (`self.CanAttack?`)
      (`self.SwordAttack`))))

(event `Attack2`
  (`/Engine/EditorBlueprintResources/StandardMacros.DoOnce` false :!label _label_2
    (:`Completed`
      (`KismetSystemLibrary.Delay` 0.1)
      (`|PlayMontage` (`self.Ref_CharacterMesh`) "/Game/Characters/RPG_Character/Animation/SwordAttack/M_Attack2.M_Attack2"
        (:`then`
          (set `self.AttackIndex` 2)
          (goto _label_2 :!via `Reset`))))))

(event `SwordAttack`
  (if (`self.IsAttacking`)
    (set `self.SaveAttack` true)
    (else
      (set `self.IsAttacking` true)
      (switch `int` (`self.AttackIndex`) :!label _label_3
        (:`0`
          (`self.Attack1`))
        (:`1`
          (`self.Attack2`))
        (:`2`
          (`self.AttackKick`))
        (:`3`
          (`self.Attack3`))))))

(event `AttackKick`
  (`/Engine/EditorBlueprintResources/StandardMacros.DoOnce` false :!label _label_4
    (:`Completed`
      (`KismetSystemLibrary.Delay` 0.1)
      (`|PlayMontage` (`self.Ref_CharacterMesh`) "/Game/Characters/RPG_Character/Animation/SwordAttack/M_Kick.M_Kick"
        (:`then`
          (set `self.AttackIndex` 3)
          (goto _label_4 :!via `Reset`))))))

(event `SwordAttackCombo`
  (if (`self.SaveAttack`)
    (set `self.SaveAttack` false)
    (goto _label_3)
    (else
      (`self.StopCombo`))))

(event `Attack3`
  (`/Engine/EditorBlueprintResources/StandardMacros.DoOnce` false :!label _label_5
    (:`Completed`
      (`KismetSystemLibrary.Delay` 0.1)
      (`|PlayMontage` (`self.Ref_CharacterMesh`) "/Game/Characters/RPG_Character/Animation/SwordAttack/M_Attack3.M_Attack3"
        (:`then`
          (set `self.AttackIndex` 4)
          (goto _label_5 :!via `Reset`))))))

(event `StopCombo`
  (set `self.IsAttacking` false)
  (set `self.AttackIndex` 0))