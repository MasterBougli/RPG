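; Player stats component for BP_ThirdPersonCharacter that holds health, stamina, hunger, thirst, XP and level.
; Each survival stat has functions to raise or lower its clamped current value and its maximum, with decreases returning whether zero is reached.
; XP overflow raises the level and scales the next threshold up, recursing to handle multiple level-ups.
; BeginPlay caches the owning character and its HUD reference, which the stat functions never use.
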(event `self.ReceiveBeginPlay`
  (bind _asbp_third_person_character (cast `/Game/ThirdPerson/Blueprints/BP_ThirdPersonCharacter` (`self.GetOwner`)))
  (bind _output_get (set `self.As BP Third Person Character` _asbp_third_person_character))
  (set `self.Ref HUD` (`/Game/ThirdPerson/Blueprints/BP_ThirdPersonCharacter.Ref_HUD` _output_get)))

(fn `Decrease Health`
  (params (Amount :type "Float (double-precision)"))
  (returns (IsDead :type Boolean))
  (locals (L_Amount :type "Float (double-precision)"))
  (set `local.L_Amount` Amount)
  (set `self.HealthCurrent` (`KismetMathLibrary.FClamp` (- (`self.HealthCurrent`) (`local.L_Amount`)) 0.0 (`self.HealthMax`)))
  (return (== (`self.HealthCurrent`) 0.0)))

(fn `Decrease HealthMax`
  (params (Amount :type "Float (double-precision)"))
  (returns (IsDead :type Boolean))
  (locals (L_Amount :type "Float (double-precision)"))
  (set `local.L_Amount` Amount)
  (set `self.HealthMax` (`KismetMathLibrary.FClamp` (- (`self.HealthMax`) (`local.L_Amount`)) 0.0 (`self.HealthMax`)))
  (return (<= (`self.HealthMax`) 0.0)))

(fn `Decrease Hunger`
  (params (Amount :type "Float (double-precision)"))
  (returns (Starving :type Boolean))
  (locals (L_Amount :type "Float (double-precision)"))
  (set `local.L_Amount` Amount)
  (set `self.HungerCurrent` (`KismetMathLibrary.FClamp` (- (`self.HungerCurrent`) (`local.L_Amount`)) 0.0 (`self.HungerMax`)))
  (return (<= (`self.HungerCurrent`) 0.0)))

(fn `Decrease HungerMax`
  (params (Amount :type "Float (double-precision)"))
  (returns (Starving :type Boolean))
  (locals (L_Amount :type "Float (double-precision)"))
  (set `local.L_Amount` Amount)
  (set `self.HungerMax` (`KismetMathLibrary.FClamp` (- (`self.HungerMax`) (`local.L_Amount`)) 0.0 (`self.HungerMax`)))
  (return (<= (`self.HungerMax`) 0.0)))

(fn `Decrease Stamina`
  (params (Amount :type "Float (double-precision)"))
  (returns (NoStam :type Boolean))
  (locals (L_Amount :type "Float (double-precision)"))
  (set `local.L_Amount` Amount)
  (set `self.StaminaCurrent` (`KismetMathLibrary.FClamp` (- (`self.StaminaCurrent`) (`local.L_Amount`)) 0.0 (`self.StaminaMax`)))
  (return (<= (`self.StaminaCurrent`) 0.0)))

(fn `Decrease StaminaMax`
  (params (Amount :type "Float (double-precision)"))
  (returns (NoStam :type Boolean))
  (locals (L_Amount :type "Float (double-precision)"))
  (set `local.L_Amount` Amount)
  (set `self.StaminaMax` (`KismetMathLibrary.FClamp` (- (`self.StaminaMax`) (`local.L_Amount`)) 0.0 (`self.StaminaMax`)))
  (return (<= (`self.StaminaMax`) 0.0)))

(fn `Decrease Thirst`
  (params (Amount :type "Float (double-precision)"))
  (returns (Thirsty :type Boolean))
  (locals (L_Amount :type "Float (double-precision)"))
  (set `local.L_Amount` Amount)
  (set `self.ThirstCurrent` (`KismetMathLibrary.FClamp` (- (`self.ThirstCurrent`) (`local.L_Amount`)) 0.0 (`self.ThirstMax`)))
  (return (<= (`self.ThirstCurrent`) 0.0)))

(fn `Decrease ThirstMax`
  (params (Amount :type "Float (double-precision)"))
  (returns (Thirsty :type Boolean))
  (locals (L_Amount :type "Float (double-precision)"))
  (set `local.L_Amount` Amount)
  (set `self.ThirstMax` (`KismetMathLibrary.FClamp` (- (`self.ThirstMax`) (`local.L_Amount`)) 0.0 (`self.ThirstMax`)))
  (return (<= (`self.ThirstMax`) 0.0)))

(fn `Increase Health`
  (params (Amount :type "Float (double-precision)"))
  (locals (L_Amount :type "Float (double-precision)"))
  (set `local.L_Amount` Amount)
  (set `self.HealthCurrent` (`KismetMathLibrary.FClamp` (+ (`self.HealthCurrent`) (`local.L_Amount`)) 0.0 (`self.HealthMax`))))

(fn `Increase HealthMax`
  (params (Amount :type "Float (double-precision)"))
  (locals (L_Amount :type "Float (double-precision)"))
  (set `local.L_Amount` Amount)
  (set `self.HealthMax` (+ (`self.HealthMax`) (`local.L_Amount`))))

(fn `Increase Hunger`
  (params (Amount :type "Float (double-precision)"))
  (locals (L_Amount :type "Float (double-precision)"))
  (set `local.L_Amount` Amount)
  (set `self.HungerCurrent` (`KismetMathLibrary.FClamp` (+ (`self.HungerCurrent`) (`local.L_Amount`)) 0.0 (`self.HungerMax`))))

(fn `Increase HungerMax`
  (params (Amount :type "Float (double-precision)"))
  (locals (L_Amount :type "Float (double-precision)"))
  (set `local.L_Amount` Amount)
  (set `self.HungerMax` (+ (`self.HungerMax`) (`local.L_Amount`))))

(fn `Increase Stamina`
  (params (Amount :type "Float (double-precision)"))
  (locals (L_Amount :type "Float (double-precision)"))
  (set `local.L_Amount` Amount)
  (set `self.StaminaCurrent` (`KismetMathLibrary.FClamp` (+ (`self.StaminaCurrent`) (`local.L_Amount`)) 0.0 (`self.StaminaMax`))))

(fn `Increase StaminaMax`
  (params (Amount :type "Float (double-precision)"))
  (locals (L_Amount :type "Float (double-precision)"))
  (set `local.L_Amount` Amount)
  (set `self.StaminaMax` (+ (`self.StaminaMax`) (`local.L_Amount`))))

(fn `Increase Thirst`
  (params (Amount :type "Float (double-precision)"))
  (locals (L_Amount :type "Float (double-precision)"))
  (set `local.L_Amount` Amount)
  (set `self.ThirstCurrent` (`KismetMathLibrary.FClamp` (+ (`self.ThirstCurrent`) (`local.L_Amount`)) 0.0 (`self.ThirstMax`))))

(fn `Increase ThirstMax`
  (params (Amount :type "Float (double-precision)"))
  (locals (L_Amount :type "Float (double-precision)"))
  (set `local.L_Amount` Amount)
  (set `self.ThirstMax` (+ (`self.ThirstMax`) (`local.L_Amount`))))

(fn `IncreaseLevel`
  (params (Amount :type Integer))
  (set `self.Level` (+ Amount (`self.Level`))))

(fn `IncreaseXP`
  (params (Amount :type Integer))
  (locals (L_XpNew :type Integer) (L_Amount :type Integer) (L_ToAddAfterLevelUp :type Integer))
  (bind _output_get (set `self.XpCurrent` (+ Amount (`self.XpCurrent`))))
  (if (>= _output_get (`self.XpMax`))
    (set `self.XpCurrent` (- (`self.XpCurrent`) (`self.XpMax`)))
    (set `self.XpMax` (`KismetMathLibrary.FTrunc` (* (`KismetMathLibrary.Conv_IntToDouble` (`self.XpMax`)) 1.2)))
    (`self.IncreaseLevel` 1)
    (if (>= (`self.XpCurrent`) (`self.XpMax`))
      (`self.IncreaseXP` 0))))