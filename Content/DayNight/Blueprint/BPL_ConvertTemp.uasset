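; Blueprint function library in the DayNight folder that converts temperature values between Fahrenheit, Celsius and a custom scale called Dehss.
; Each function is a standalone arithmetic formula that takes one input temperature and returns the converted value.
; Dehss is a fixed offset from Celsius, and only conversions into it are provided, with the Fahrenheit version repeating the Celsius formula inline.
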(fn `CelsiusToDehss`
  (params (InputTemp :type "Float (double-precision)"))
  (returns (OutputTemp :type "Float (double-precision)"))
  (return (- InputTemp 37.5)))

(fn `CelsiusToFahrenheit`
  (params (InputTemp :type "Float (double-precision)"))
  (returns (OutputTemp :type "Float (double-precision)"))
  (return (+ (* InputTemp (/ 9.0 5.0)) 32.0)))

(fn `FahrenheitToCelsius`
  (params (InputTemp :type "Float (double-precision)"))
  (returns (ReturnValue :type "Float (double-precision)"))
  (return (* (- InputTemp 32.0) (/ 5.0 9.0))))

(fn `FahrenheitToDehss`
  (params (InputTemp :type "Float (double-precision)"))
  (returns (OutputTemp :type "Float (double-precision)"))
  (return (- (* (- InputTemp 32.0) (/ 5.0 9.0)) 37.5)))