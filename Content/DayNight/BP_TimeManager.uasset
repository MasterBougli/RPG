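; BP_TimeManager is a day/night time manager that stores the time of day in seconds.
; BeginPlay sets a non-looping timer with a delay of one over AmountToTickASecond, so the update fires only once as wired.
; The timer event adds AmountToAddPerTick to TimeOfDayInSeconds and resets it to zero on reaching a full day's worth of seconds.
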(event `self.ReceiveBeginPlay`
  (`KismetSystemLibrary.K2_SetTimerDelegate` (delegate `CustomEvent`) (/ 1.0 (`self.AmountToTickASecond`))))

(event `CustomEvent`
  (set `self.TimeOfDayInSeconds` (+ (`self.TimeOfDayInSeconds`) (`self.AmountToAddPerTick`)))
  (if (>= (`self.TimeOfDayInSeconds`) 86400)
    (set `self.TimeOfDayInSeconds` 0)))

(fn `UserConstructionScript`)